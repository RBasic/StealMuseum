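; Player controller for the session setup screen, where a player hosts a multiplayer game.
; On BeginPlay it adds the HUD_Param_Session widget to the viewport and shows the cursor in Game and UI input mode, locked to the window.
; The Héberger event creates an Advanced Session with the given connection count and server name as an extra setting, then opens Lobby_Map as a listen server on success.
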(event Custom|HUD%20Menu
  ;[1 1 1] HUD Menu
  (Utilities|IsValid (Variables|Default|GetHUD_Menu)
    (:Is%20Not%20Valid
      (bind _returnvalue (UserInterface|CreateWidget "/Game/HUD/HUD_Param_Session.HUD_Param_Session_C"))
      (bind _output_get (Variables|Default|SetParam%20session _returnvalue))
      (UserInterface|Viewport|AddtoViewport _output_get 0))))

(event Custom|Init%20Cursor
  ;[1 1 1] Init Cursor
  (Variables|Default|SetbShowMouseCursor true)
  (Input|SetInputModeGameandUI self 0 "LockAlways" false))

(event Custom|Héberger
  (params (Session%20Name :type String) (PublicConnections :type Integer))
  ;[1 1 1] Héberger
  (|AdvancedSession (Utilities|Array|MakeArray (Class|AdvancedSessionsLibrary|MakeLiteralSessionPropertyString "servername" Session%20Name)) self PublicConnections 0 false true false true true false false false true
    (:OnSuccess
      (Game|OpenLevel(byName) "Lobby_Map" true "listen"))))

(event EventBeginPlay
  ;[1 1 1] Init
  (CallFunction|HUDMenu)
  (CallFunction|InitCursor))

(fn ConstructionScript)