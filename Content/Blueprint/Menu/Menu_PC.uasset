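; Main-menu PlayerController that shows the HUD_Menu widget with a visible, locked cursor and handles multiplayer hosting and joining.
; Hosting opens Param_Map as a listen server, while joining works either by IP through an "open" console command or through a selected session result.
; Searching uses Advanced Sessions to refill the menu's SessionBox with one HUD_Session widget per result, tracking progress in IsFindingSession.
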(event Custom|HUD%20Menu
  ;[1 1 1] HUD Menu
  (Utilities|IsValid (Variables|Default|GetHUD_Menu)
    (:Is%20Not%20Valid
      (bind _returnvalue (UserInterface|CreateWidget "/Game/HUD/HUD_Menu.HUD_Menu_C"))
      (bind _output_get (Variables|Default|SetHUD_Menu _returnvalue))
      (UserInterface|Viewport|AddtoViewport _output_get 0))))

(event Custom|Init%20Cursor
  ;[1 1 1] Init Cursor
  (Variables|Default|SetbShowMouseCursor true)
  (Input|SetInputModeGameandUI self 0 "LockAlways" false))

(event Custom|Héberger
  ;[1 1 1] Héberger
  (Game|OpenLevel(byName) "Param_Map" true "listen"))

(event Custom|Rejoindre
  (params (IP :type String))
  ;[1 1 1] Rejoindre
  (Development|ExecuteConsoleCommand (Utilities|String|Append "open " IP) 0))

(event Custom|Rechercher
  ;[1 1 1] Rechercher
  (Widget|Panel|ClearChildren (Variables|/Game/HUD/HUD_Menu.HUD_Menu_C|GetSessionBox (Variables|Default|GetHUD_Menu)))
  (Variables|Default|SetIsFindingSession true)
  (bind _results (|FindSessionsAdvanced self 99 false "AllServers" 0 false false false)
    (:OnSuccess
      (for _array_element _results
        (bind _returnvalue (UserInterface|CreateWidget "/Game/HUD/HUD_Session.HUD_Session_C" 0 _array_element))
        (Widget|Panel|AddChild (Variables|/Game/HUD/HUD_Menu.HUD_Menu_C|GetSessionBox (Variables|Default|GetHUD_Menu)) _returnvalue))
      (Variables|Default|SetIsFindingSession false))))

(event Custom|JoinSession
  (params (SearchResult :type Blueprint%20Session%20Result%20Structure%20%28by%20ref%29))
  ;[1 1 1] Join session
  (|JoinSession self SearchResult))

(event EventBeginPlay
  ;[1 1 1] Init
  (CallFunction|HUDMenu)
  (CallFunction|InitCursor))

(fn ConstructionScript)